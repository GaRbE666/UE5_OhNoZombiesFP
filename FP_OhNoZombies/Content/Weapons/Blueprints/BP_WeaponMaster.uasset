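; BP_WeaponMaster is a weapon Blueprint, named as a master class, that provides procedural recoil motion for its Gun component.
; SetRecoilVariables caches the gun's current relative pitch and X position, then derives kicked targets from RecoilAmount and PullbackAmount.
; RecoilAnimation lerps pitch and X between those values using an Alpha input, leaving other axes untouched.
; The event graph and construction script are empty, and neither function is called here.
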(fn `RecoilAnimation`
  (params (Alpha :type "Float (double-precision)"))
  (bind (_relativerotation_roll _relativerotation_pitch _relativerotation_yaw) (`KismetMathLibrary.BreakRotator` (`SceneComponent.RelativeRotation` (`self.Gun`))))
  (bind (_relativelocation_x _relativelocation_y _relativelocation_z) (`KismetMathLibrary.BreakVector` (`SceneComponent.RelativeLocation` (`self.Gun`))))
  (`SceneComponent.K2_SetRelativeRotation` (`self.Gun`) (`KismetMathLibrary.MakeRotator` _relativerotation_roll (`KismetMathLibrary.Lerp` (`self.Pre Recoil Rot`) (`self.Recoil Rot Amount`) Alpha) _relativerotation_yaw) false false)
  (`SceneComponent.K2_SetRelativeLocation` (`self.Gun`) (`KismetMathLibrary.MakeVector` (`KismetMathLibrary.Lerp` (`self.Pre Recoil Loc`) (`self.Recoil Loc Amount`) Alpha) _relativelocation_y _relativelocation_z) false false))

(fn `Set Recoil Variables`
  (bind (_relativerotation_roll _relativerotation_pitch) (`KismetMathLibrary.BreakRotator` (`SceneComponent.RelativeRotation` (`self.Gun`))))
  (bind _relativelocation_x (`KismetMathLibrary.BreakVector` (`SceneComponent.RelativeLocation` (`self.Gun`))))
  (set `self.Pre Recoil Rot` _relativerotation_pitch)
  (set `self.Recoil Rot Amount` (+ _relativerotation_pitch (`self.Recoil Amount`)))
  (set `self.Pre Recoil Loc` _relativelocation_x)
  (set `self.Recoil Loc Amount` (+ _relativelocation_x (* (`self.Pullback Amount`) -1.0))))

(fn `UserConstructionScript`)