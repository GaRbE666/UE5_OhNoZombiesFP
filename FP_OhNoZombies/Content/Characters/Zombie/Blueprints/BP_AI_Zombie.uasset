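; Zombie enemy for a wave-style shooter that hurts the player on damage-sphere overlap and briefly pauses health recovery.
; TakeDamage scales damage by bone, awards points per hit or kill using GM_Zombies power-up states, and ragdolls the corpse with an impulse.
; InstaKill holds health at 1 via Tick.
; Death calls SelectRandomPowerUp, whose selection is hard-coded to the PointsUp case, where the spawn has no class set.
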(event `self.ReceiveBeginPlay`
  (bind _asbp_player (cast `/Game/Characters/Player/BP_Player` (`GameplayStatics.GetPlayerCharacter` 0)))
  (set `self.Player Ref` _asbp_player)
  (bind _asgm_zombies (cast `/Game/Blueprints/GameModes/GM_Zombies` (`GameplayStatics.GetGameMode`)))
  (set `self.GM Zombies Ref` _asgm_zombies))

(event `self.ReceiveTick`
  (params (DeltaSeconds :type "Float (single-precision)"))
  (if (`/Game/Blueprints/GameModes/GM_Zombies.InstaKill Is Active` (`self.GM Zombies Ref`))
    (set `/Game/Blueprints/Components/BPC_Health.Current Health` 1.0 (`self.BPC_Health`))))

(event `self.DamageSphere.OnComponentBeginOverlap`
  (params (OverlappedComponent :type "PrimitiveComponent Object Reference") (OtherActor :type "Actor Object Reference") (OtherComp :type "PrimitiveComponent Object Reference") (OtherBodyIndex :type Integer) (bFromSweep :type Boolean) (SweepResult :type "HitResult Structure (by ref)"))
  (bind _bpc_health (`/Game/Characters/Player/BP_Player.BPC_Health` (`self.Player Ref`)))
  (if (`self.canDamage`)
    (bind _asbp_player (cast `/Game/Characters/Player/BP_Player` OtherActor))
    (if (not (`/Game/Characters/Player/BP_Player.isDead` _asbp_player))
      (`/Game/Characters/Player/BP_Player.Take Damage` _asbp_player 10.0 self)
      (set `/Game/Blueprints/Components/BPC_Health.isWaitingToRecover` true _bpc_health)
      (`KismetSystemLibrary.Delay` 1.5)
      (set `/Game/Blueprints/Components/BPC_Health.isWaitingToRecover` false _bpc_health))))

(fn `Select Random PowerUp`
  (bind (_returnvalue_location _returnvalue_rotation) (`KismetMathLibrary.BreakTransform` (`self.GetTransform`)))
  (bind (_returnvalue_location_2 _returnvalue_rotation_2) (`KismetMathLibrary.BreakTransform` (`self.GetTransform`)))
  (bind (_returnvalue_location_3 _returnvalue_rotation_3) (`KismetMathLibrary.BreakTransform` (`self.GetTransform`)))
  (bind (_returnvalue_location_4 _returnvalue_rotation_4) (`KismetMathLibrary.BreakTransform` (`self.GetTransform`)))
  (if (> (`KismetMathLibrary.RandomFloatInRange` 0.0 1.0) 0.0)
    (switch `int` 4
      (:`0`
        (`|SpawnActorFromClass` "/Game/Blueprints/IteractableItems/PowerUps/BP_PowerUp.BP_PowerUp_C" (`KismetMathLibrary.MakeTransform` _returnvalue_location_3 _returnvalue_rotation_3) "Undefined" "OverrideRootScale" null null "NewEnumerator0" null)
        (`KismetSystemLibrary.PrintString` "InstaKill"))
      (:`1`
        (`|SpawnActorFromClass` "/Game/Blueprints/IteractableItems/PowerUps/BP_PowerUp.BP_PowerUp_C" (`KismetMathLibrary.MakeTransform` _returnvalue_location _returnvalue_rotation) "Undefined" "OverrideRootScale" null null "NewEnumerator1" null)
        (`KismetSystemLibrary.PrintString` "Kaboom"))
      (:`2`
        (`|SpawnActorFromClass` "/Game/Blueprints/IteractableItems/PowerUps/BP_PowerUp.BP_PowerUp_C" (`KismetMathLibrary.MakeTransform` _returnvalue_location_4 _returnvalue_rotation_4) "Undefined" "OverrideRootScale" null null "NewEnumerator2" null)
        (`KismetSystemLibrary.PrintString` "DoublePoints"))
      (:`4`
        (`|SpawnActorFromClass` "/Game/Blueprints/IteractableItems/PowerUps/BP_PowerUp.BP_PowerUp_C" (`KismetMathLibrary.MakeTransform` _returnvalue_location_2 _returnvalue_rotation_2) "Undefined" "OverrideRootScale" null null "NewEnumerator4" null)
        (`KismetSystemLibrary.PrintString` "PointsUp")))))

(fn `TakeDamage`
  (params (Amount :type "Float (double-precision)") (`Bone Name` :type Name) (`Impact Point` :type "Vector Structure"))
  (returns (dead :type Boolean))
  (bind _dead (`/Game/Blueprints/Components/BPC_Health.Remove Health` (`self.BPC_Health`) (select `bool` (or (== `Bone Name` "calf_l") (== `Bone Name` "calf_r") (== `Bone Name` "foot_l") (== `Bone Name` "foot_r") (== `Bone Name` "thigh_l") (== `Bone Name` "thigh_r")) :`false` (select `bool` (== `Bone Name` "head") :`false` Amount :`true` (* Amount 2.0)) :`true` (* Amount 0.8))))
  (if _dead
    ;[1 1 1] Physic Death
    (`PrimitiveComponent.SetSimulatePhysics` (`self.Mesh`) true)
    (`PrimitiveComponent.SetCollisionEnabled` (`self.CapsuleComponent`) "NoCollision")
    (`PrimitiveComponent.SetCollisionResponseToChannel` (`self.Mesh`) "ECC_Visibility" "ECR_Ignore")
    (`PrimitiveComponent.AddImpulse` (`self.Mesh`) (* `Impact Point` -10000.0) `Bone Name` false)
    (bind _asgm_zombies (cast `/Game/Blueprints/GameModes/GM_Zombies` (`GameplayStatics.GetGameMode`)))
    (`/Engine/EditorBlueprintResources/StandardMacros.IncrementInt` (`/Game/Blueprints/GameModes/GM_Zombies.Zombies Dead` _asgm_zombies)
      (:`  `
        (if (`/Game/Blueprints/GameModes/GM_Zombies.Kaboom Is Active` _asgm_zombies)
          (`/Game/Characters/Player/BP_Player.AddPoints` (`self.Player Ref`) 500)
          (elif (`/Game/Blueprints/GameModes/GM_Zombies.Double Points Is Active` _asgm_zombies)
            (`/Game/Characters/Player/BP_Player.AddPoints` (`self.Player Ref`) (* (`self.PointsDead`) 2))
            (else
              (`/Game/Characters/Player/BP_Player.AddPoints` (`self.Player Ref`) (`self.PointsDead`)))))
        (`PrimitiveComponent.SetCollisionEnabled` (`self.DamageSphere`) "NoCollision")
        (`self.Select Random PowerUp`)
        (set `self.PointsPerHit` 10)
        (`self.SetLifeSpan` 10.0)
        (return true)))
    (else
      ;[1 1 1] Add Player points
      (bind _asbp_player (cast `/Game/Characters/Player/BP_Player` (`GameplayStatics.GetPlayerCharacter` 0)))
      (bind _asgm_zombies_2 (cast `/Game/Blueprints/GameModes/GM_Zombies` (`GameplayStatics.GetGameMode`)))
      (if (`/Game/Blueprints/GameModes/GM_Zombies.Double Points Is Active` _asgm_zombies_2)
        (`/Game/Characters/Player/BP_Player.AddPoints` _asbp_player (* (`self.PointsPerHit`) 2))
        (else
          (`/Game/Characters/Player/BP_Player.AddPoints` _asbp_player (`self.PointsPerHit`)))))))

(fn `UserConstructionScript`)