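; AI controller for the zombie enemy, which starts its behavior tree BT_Zombie two seconds after spawn so the zombie waits before walking.
; Each tick it measures the distance from the controlled pawn to the player and writes the InAttackRange blackboard key for the tree.
; The key is true only while a living player is within a short fixed range, and is forced false once the player is dead.
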(event `self.ReceiveBeginPlay`
  ;[1 1 1] Delay before Zombie walk
  (`KismetSystemLibrary.Delay` 2.0)
  (`self.RunBehaviorTree` "/Game/Characters/Zombie/Blueprints/BT_Zombie.BT_Zombie"))

(event `self.ReceiveTick`
  (params (DeltaSeconds :type "Float (single-precision)"))
  (`/Engine/EditorBlueprintResources/StandardMacros.IsValid` (`AIBlueprintHelperLibrary.GetBlackboard` null)
    (:`Is Valid`
      (bind _asbp_player (cast `/Game/Characters/Player/BP_Player` (`GameplayStatics.GetPlayerCharacter` 0)))
      (if (not (`/Game/Characters/Player/BP_Player.isDead` _asbp_player))
        (`BlackboardComponent.SetValueAsBool` (`AIBlueprintHelperLibrary.GetBlackboard` null) "InAttackRange" (< (`self.GetDistanceTo` (`self.K2_GetPawn`) (`GameplayStatics.GetPlayerCharacter` 0)) 125.0))
        (else
          (`BlackboardComponent.SetValueAsBool` (`AIBlueprintHelperLibrary.GetBlackboard` null) "InAttackRange" false))))))

(fn `UserConstructionScript`)