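; Pack-a-Punch (PAP) staircase for the zombies mode that rises once every PAP access button in the level is pressed.
; BeginPlay counts the BP_AccessPAP actors, and Tick compares that total to the game mode's ButtonsPressed.
; A timeline lifts the Stairs component, and its Start Timer event track waits briefly, resets the counter and all buttons, then reverses the timeline to lower the stairs.
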(event `self.ReceiveBeginPlay`
  (bind _asgm_zombies (cast `/Game/Blueprints/GameModes/GM_Zombies` (`GameplayStatics.GetGameMode`)))
  (set `self.GM_Zombies Ref` _asgm_zombies)
  (bind _outactors (`GameplayStatics.GetAllActorsOfClass` "/Game/Blueprints/IteractableItems/BP_AccessPAP.BP_AccessPAP_C"))
  (set `self.Total Button To PAP` (`KismetArrayLibrary.Array_Length` _outactors)))

(event `self.ReceiveTick`
  (params (DeltaSeconds :type "Float (single-precision)"))
  (if (== (`/Game/Blueprints/GameModes/GM_Zombies.ButtonsPressed` (`self.GM_Zombies Ref`)) (`self.Total Button To PAP`))
    (bind (_direction _alpha) (`Timeline|UpStairs` :!label _label)
      (:`Update`
        (`SceneComponent.K2_SetRelativeLocation` (`self.Stairs`) (`KismetMathLibrary.MakeVector` 0.0 0.0 (`KismetMathLibrary.Lerp` 0.0 160.0 _alpha)) false false))
      (:`StartTimer`
        (`KismetSystemLibrary.Delay` 3.0)
        (set `/Game/Blueprints/GameModes/GM_Zombies.ButtonsPressed` 0 (`self.GM_Zombies Ref`))
        (bind _outactors (`GameplayStatics.GetAllActorsOfClass` "/Game/Blueprints/IteractableItems/BP_AccessPAP.BP_AccessPAP_C"))
        (for _array_element _outactors
          (set `/Game/Blueprints/IteractableItems/BP_AccessPAP.ButtonIsPressed` false _array_element))
        (goto _label :!via `Reverse`)))))

(fn `UserConstructionScript`)