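; Water ramp trigger that carries the player along with a water actor through the WaterRamp level sequence.
; While BP_Player overlaps the construction-positioned box, every Tick snaps them to the water actor, disables movement, attaches them and creates and plays a new sequence player.
; When the sequence finishes, the player detaches, resets capsule rotation and resumes walking, and after a delay the sequence plays in reverse.
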(event `self.ReceiveBeginPlay`
  (bind _asbp_player (cast `/Game/Characters/Player/BP_Player` (`GameplayStatics.GetPlayerCharacter` 0)))
  (set `self.Player Ref` _asbp_player))

(event `self.ReceiveTick`
  (params (DeltaSeconds :type "Float (single-precision)"))
  (if (`self.Player Enter`)
    (`self.K2_SetActorLocation` (`self.Player Ref`) (+ (`self.K2_GetActorLocation` (`self.WaterActor`)) (0.0 100.0 50.0)) false false)
    (`self.SetActorScale3D` (`self.Player Ref`) (1.0 1.0 1.0))
    (`CharacterMovementComponent.DisableMovement` (`Character.CharacterMovement` (`self.Player Ref`)))
    (`self.K2_AttachToActor` (`self.Player Ref`) (`self.WaterActor`) "None" "KeepWorld" "KeepWorld" "KeepWorld" true)
    (bind (_outactor _returnvalue) (`LevelSequencePlayer.CreateLevelSequencePlayer` "/Game/Sequences/WaterRamp.WaterRamp"))
    (bind _output_get (set `self.SequenceWaterRamp Ref` _returnvalue))
    (`MovieSceneSequencePlayer.Play` _output_get)
    (add `MovieSceneSequencePlayer.OnFinished` (`self.SequenceWaterRamp Ref`) (delegate `RampFinish`))))

(event `RampFinish`
  (`self.K2_DetachFromActor` (`self.Player Ref`) "KeepWorld" "KeepWorld" "KeepWorld")
  (`SceneComponent.K2_SetRelativeRotation` :`self` (`Character.CapsuleComponent` (`self.Player Ref`)))
  (`CharacterMovementComponent.SetMovementMode` (`Character.CharacterMovement` (`self.Player Ref`)) "MOVE_Walking" 0)
  (remove `MovieSceneSequencePlayer.OnFinished` (`self.SequenceWaterRamp Ref`) (delegate `RampFinish`))
  (`KismetSystemLibrary.Delay` 1.0)
  (`MovieSceneSequencePlayer.PlayReverse` (`self.SequenceWaterRamp Ref`)))

(event `self.Box.OnComponentBeginOverlap`
  (params (OverlappedComponent :type "PrimitiveComponent Object Reference") (OtherActor :type "Actor Object Reference") (OtherComp :type "PrimitiveComponent Object Reference") (OtherBodyIndex :type Integer) (bFromSweep :type Boolean) (SweepResult :type "HitResult Structure (by ref)"))
  (cast `/Game/Characters/Player/BP_Player` OtherActor)
  (set `self.Player Enter` true))

(event `self.Box.OnComponentEndOverlap`
  (params (OverlappedComponent :type "PrimitiveComponent Object Reference") (OtherActor :type "Actor Object Reference") (OtherComp :type "PrimitiveComponent Object Reference") (OtherBodyIndex :type Integer))
  (cast `/Game/Characters/Player/BP_Player` OtherActor)
  (set `self.Player Enter` false))

(fn `UserConstructionScript`
  (`SceneComponent.K2_SetRelativeTransform` (`self.Box`) (`self.Collision Transform`) false false))