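; Buyable perk station with a configurable mesh, name and cost, though a purchase always activates the player's Jug perk.
; Overlapping the box stores the player reference and shows a purchase prompt widget, both cleared on exit.
; Tick polls for interaction, enough points and no reload or ADS, then updates max health, removes the prompt and disables the box's collision.
; The cost is only checked, never deducted here.
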(event `self.ReceiveTick`
  (params (DeltaSeconds :type "Float (single-precision)"))
  (bind _player_ref (`self.Player Ref`))
  (`/Engine/EditorBlueprintResources/StandardMacros.IsValid` (`self.Player Ref`)
    (:`Is Valid`
      ;[1 1 1] Checks
      (if (and (`/Game/Characters/Player/BP_Player.isInteracting` _player_ref) (`/Game/Characters/Player/BP_Player.canSpendPoints` _player_ref) (>= (`/Game/Characters/Player/BP_Player.Points` (`self.Player Ref`)) (`self.Perk Cost`)))
        (if (and (`KismetSystemLibrary.IsValid` (`self.Player Ref`)) (not (`/Game/Characters/Player/BP_Player.isReloading` (`self.Player Ref`))) (not (`/Game/Characters/Player/BP_Player.isADS` (`self.Player Ref`))))
          (set `/Game/Characters/Player/BP_Player.JugIsActivated` true (`self.Player Ref`))
          (`/Game/Blueprints/Components/BPC_Health.Update Max Health` (`/Game/Characters/Player/BP_Player.BPC_Health` (`self.Player Ref`)))
          (set `/Game/Characters/Player/BP_Player.canSpendPoints` false (`self.Player Ref`))
          (`Widget.RemoveFromParent` (`self.WB Text Ref`))
          (`PrimitiveComponent.SetCollisionEnabled` (`self.Box`) "NoCollision"))))))

(event `self.Box.OnComponentBeginOverlap`
  (params (OverlappedComponent :type "PrimitiveComponent Object Reference") (OtherActor :type "Actor Object Reference") (OtherComp :type "PrimitiveComponent Object Reference") (OtherBodyIndex :type Integer) (bFromSweep :type Boolean) (SweepResult :type "HitResult Structure (by ref)"))
  (bind _asbp_player (cast `/Game/Characters/Player/BP_Player` OtherActor))
  (set `self.Player Ref` _asbp_player)
  (set `/Game/Characters/Player/BP_Player.canSpendPoints` true _asbp_player)
  (bind _returnvalue (`|CreateWidget` "/Game/Blueprints/Widgets/WB_Text.WB_Text_C"))
  (set `self.WB Text Ref` _returnvalue)
  (`UserWidget.AddToViewport` _returnvalue 0)
  (`TextBlock.SetText` (`/Game/Blueprints/Widgets/WB_Text.BuyableText` (`self.WB Text Ref`)) (`|FormatText` "Press F to buy {PerkName} ({PerkCost})" (`self.Perk Name`) (`self.Perk Cost`))))

(event `self.Box.OnComponentEndOverlap`
  (params (OverlappedComponent :type "PrimitiveComponent Object Reference") (OtherActor :type "Actor Object Reference") (OtherComp :type "PrimitiveComponent Object Reference") (OtherBodyIndex :type Integer))
  (bind _asbp_player (cast `/Game/Characters/Player/BP_Player` OtherActor))
  (set `self.Player Ref` null)
  (set `/Game/Characters/Player/BP_Player.canSpendPoints` false _asbp_player)
  (`/Engine/EditorBlueprintResources/StandardMacros.IsValid` (`self.WB Text Ref`)
    (:`Is Valid`
      (`Widget.RemoveFromParent` (`self.WB Text Ref`)))))

(fn `UserConstructionScript`
  (`StaticMeshComponent.SetStaticMesh` (`self.StaticMesh`) (`self.Mesh`)))