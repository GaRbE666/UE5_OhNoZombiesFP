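; Point-purchase interactable that works as either a buyable door or a weapon buy, selected by IsDoor.
; Box overlap caches the BP_Player, enables spending and shows a cost prompt widget; leaving reverses this.
; Tick polls for interaction and sufficient points, then either adds WeaponClass unless already owned, or plays a timeline.
; The timeline lowers the door, with tracks that disable collision, clear the prompt and deduct points, then destroys the actor.
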(event `self.ReceiveBeginPlay`
  (`StaticMeshComponent.SetStaticMesh` (`self.Door`) (`self.Mesh`)))

(event `self.ReceiveTick`
  (params (DeltaSeconds :type "Float (single-precision)"))
  (bind _playerref (`self.PlayerRef`))
  (`/Engine/EditorBlueprintResources/StandardMacros.IsValid` (`self.PlayerRef`)
    (:`Is Valid`
      ;[1 1 1] Checks
      (if (and (`/Game/Characters/Player/BP_Player.isInteracting` _playerref) (`/Game/Characters/Player/BP_Player.canSpendPoints` _playerref) (>= (`/Game/Characters/Player/BP_Player.Points` _playerref) (`self.Object Cost`)))
        (if (`self.isDoor`)
          (bind (_direction _alpha) (`Timeline|OpenDoorTL`)
            (:`Update`
              (`SceneComponent.K2_SetRelativeLocation` (`self.Door`) (`KismetMathLibrary.MakeVector` 0.0 0.0 (`KismetMathLibrary.Lerp` 0.0 -250.0 _alpha)) false false))
            (:`Finished`
              (`self.K2_DestroyActor`))
            (:`DisableCollision`
              (`PrimitiveComponent.SetCollisionEnabled` (`self.Door`) "NoCollision"))
            (:`DisableText`
              (`Widget.RemoveFromParent` (`self.WBDoorTextRef`)))
            (:`RemovePoints`
              (`/Game/Characters/Player/BP_Player.RemovePoints` (`self.PlayerRef`) (`self.Object Cost`))))
          (elif (`self.Check If Weapon Are Equiped`)
            (`KismetSystemLibrary.PrintString` "No lo puedo comprar")
            (else
              (`self.Add Weapon To Player`))))))))

(event `self.Box.OnComponentBeginOverlap`
  (params (OverlappedComponent :type "PrimitiveComponent Object Reference") (OtherActor :type "Actor Object Reference") (OtherComp :type "PrimitiveComponent Object Reference") (OtherBodyIndex :type Integer) (bFromSweep :type Boolean) (SweepResult :type "HitResult Structure (by ref)"))
  (bind _asbp_player (cast `/Game/Characters/Player/BP_Player` OtherActor))
  (set `self.PlayerRef` _asbp_player)
  (set `/Game/Characters/Player/BP_Player.canSpendPoints` true _asbp_player)
  (bind _returnvalue (`|CreateWidget` "/Game/Blueprints/Widgets/WB_DoorText.WB_DoorText_C"))
  (set `self.WBDoorTextRef` _returnvalue)
  (`UserWidget.AddToViewport` _returnvalue 0)
  (if (`self.isDoor`)
    (`TextBlock.SetText` (`/Game/Blueprints/Widgets/WB_DoorText.DoorText` (`self.WBDoorTextRef`)) (`|FormatText` "Press F to open door ( {doorCost})" (`self.Object Cost`)))
    (else
      (`TextBlock.SetText` (`/Game/Blueprints/Widgets/WB_DoorText.DoorText` (`self.WBDoorTextRef`)) (`|FormatText` "Press F to buy gun ({objectCost})" (`self.Object Cost`))))))

(event `self.Box.OnComponentEndOverlap`
  (params (OverlappedComponent :type "PrimitiveComponent Object Reference") (OtherActor :type "Actor Object Reference") (OtherComp :type "PrimitiveComponent Object Reference") (OtherBodyIndex :type Integer))
  (bind _asbp_player (cast `/Game/Characters/Player/BP_Player` OtherActor))
  (set `self.PlayerRef` null)
  (set `/Game/Characters/Player/BP_Player.canSpendPoints` false _asbp_player)
  (`Widget.RemoveFromParent` (`self.WBDoorTextRef`)))

(fn `Add Weapon To Player`
  (`KismetArrayLibrary.Array_Add` (`/Game/Characters/Player/BP_Player.WeaponsEquiped` (`self.PlayerRef`)) (`self.WeaponClass`))
  (`Widget.RemoveFromParent` (`self.WBDoorTextRef`))
  (`/Game/Characters/Player/BP_Player.RemovePoints` (`self.PlayerRef`) (`self.Object Cost`)))

(fn `Check If Weapon Are Equiped`
  (returns (ReturnValue :type Boolean))
  (bind _weaponsequiped (`/Game/Characters/Player/BP_Player.WeaponsEquiped` (`self.PlayerRef`)))
  (return (`KismetArrayLibrary.Array_IsValidIndex` _weaponsequiped (`KismetArrayLibrary.Array_Find` _weaponsequiped (`self.WeaponClass`)))))

(fn `Set Text To Show`
  (params (Text :type Text)))

(fn `UserConstructionScript`)