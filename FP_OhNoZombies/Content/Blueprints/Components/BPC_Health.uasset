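; BPC_Health is a player health component that tracks current and maximum health and regenerates it over time.
; On BeginPlay it casts its owner to BP_Player and initializes health, raising the maximum if the player's Jug flag is active.
; Tick restores health in small timed increments while it is below maximum and recovery is not paused.
; Add and remove functions clamp the value, with removal reporting whether health reached zero.
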(event `self.ReceiveBeginPlay`
  (bind _asbp_player (cast `/Game/Characters/Player/BP_Player` (`self.GetOwner`)))
  (set `self.Player Ref` _asbp_player)
  (`self.Update Max Health`)
  (`KismetSystemLibrary.PrintString` (`KismetSystemLibrary.GetDisplayName` _asbp_player)))

(event `self.ReceiveTick`
  (params (DeltaSeconds :type "Float (single-precision)"))
  (bind _returnvalue (+ DeltaSeconds (`self.Time To Recover Health`)))
  ;[1 1 1] Recover Health by time
  (if (and (< (`self.Current Health`) (`self.Max Health`)) (not (`self.isWaitingToRecover`)))
    (set `self.canRecoverHealth` true)
    (else
      (set `self.canRecoverHealth` false)))
  (if (`self.canRecoverHealth`)
    (if (>= _returnvalue 0.1)
      (set `self.Time To Recover Health` 0.0)
      (`self.Add Health` 1.0)
      (else
        (set `self.Time To Recover Health` _returnvalue)))))

(fn `Add Health`
  (params (Amount :type "Float (double-precision)"))
  (set `self.Current Health` (`KismetMathLibrary.FClamp` (+ Amount (`self.Current Health`)) 0.0 (`self.Max Health`))))

(fn `Remove Health`
  (params (Amount :type "Float (double-precision)"))
  (returns (Dead :type Boolean))
  (bind _output_get (set `self.Current Health` (`KismetMathLibrary.FClamp` (- (`self.Current Health`) Amount) 0.0 (`self.Max Health`))))
  (return (<= _output_get 0.0)))

(fn `Update Max Health`
  (if (`/Game/Characters/Player/BP_Player.JugIsActivated` (`self.Player Ref`))
    (bind _output_get (set `self.Max Health` (+ (`self.Max Health`) 20.0)))
    (set `self.Current Health` _output_get)
    (else
      (set `self.Current Health` (`self.Max Health`)))))