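; BP_Vagon is a purchasable wagon ride: the player pays points to be carried along a sequenced path and then ejected.
; A trigger box shows the cost prompt and allows spending; Tick polls the player's interact state and point balance.
; On purchase, the player is attached with movement disabled while a Level Sequence plays.
; Its finish event detaches the player, plays an expulsion sequence, restores walking, then reverses the wagon sequence after a delay.
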(event `self.ReceiveBeginPlay`
  (bind _asbp_player (cast `/Game/Characters/Player/BP_Player` (`GameplayStatics.GetPlayerCharacter` 0)))
  (set `self.Player Ref` _asbp_player))

(event `self.ReceiveTick`
  (params (DeltaSeconds :type "Float (single-precision)"))
  (bind _player_ref (`self.Player Ref`))
  (if (and (`/Game/Characters/Player/BP_Player.isInteracting` _player_ref) (`/Game/Characters/Player/BP_Player.canSpendPoints` _player_ref) (>= (`/Game/Characters/Player/BP_Player.Points` (`self.Player Ref`)) (`self.Wagon Cost`)))
    (if (`self.isWagon`)
      (`/Game/Characters/Player/BP_Player.RemovePoints` (`self.Player Ref`) (`self.Wagon Cost`))
      ;[1 1 1] Vagon Anim
      (`self.K2_SetActorLocation` (`self.Player Ref`) (+ (`self.K2_GetActorLocation` (`self.Vagon`)) (0.0 0.0 100.0)) false false)
      (`CharacterMovementComponent.DisableMovement` (`Character.CharacterMovement` (`self.Player Ref`)))
      (`self.K2_AttachToActor` (`self.Player Ref`) (`self.Vagon`) "None" "KeepWorld" "KeepWorld" "KeepWorld" true)
      (bind (_outactor _returnvalue) (`LevelSequencePlayer.CreateLevelSequencePlayer` "/Game/VagonAnim.VagonAnim"))
      (`MovieSceneSequencePlayer.Play` _returnvalue)
      (add `MovieSceneSequencePlayer.OnFinished` _returnvalue (delegate `ExpulseFromVagon`)))))

(event `ExpulseFromVagon`
  ;[1 1 1] Vagon Anim
  (`self.K2_DetachFromActor` (`self.Player Ref`) "KeepWorld" "KeepWorld" "KeepWorld")
  (bind (_outactor _returnvalue) (`LevelSequencePlayer.CreateLevelSequencePlayer` "/Game/Expulse.Expulse"))
  (`MovieSceneSequencePlayer.Play` _returnvalue)
  (`CharacterMovementComponent.SetMovementMode` (`Character.CharacterMovement` (`self.Player Ref`)) "MOVE_Walking" 0)
  (`KismetSystemLibrary.Delay` 2.0)
  (`MovieSceneSequencePlayer.PlayReverse` (stale `self.ReceiveTick` _returnvalue))
  (remove `MovieSceneSequencePlayer.OnFinished` (stale `self.ReceiveTick` _returnvalue) (delegate `ExpulseFromVagon`)))

(event `self.Box.OnComponentBeginOverlap`
  (params (OverlappedComponent :type "PrimitiveComponent Object Reference") (OtherActor :type "Actor Object Reference") (OtherComp :type "PrimitiveComponent Object Reference") (OtherBodyIndex :type Integer) (bFromSweep :type Boolean) (SweepResult :type "HitResult Structure (by ref)"))
  (cast `/Game/Characters/Player/BP_Player` OtherActor)
  (set `/Game/Characters/Player/BP_Player.canSpendPoints` true (`self.Player Ref`))
  (set `self.isWagon` true)
  (bind _returnvalue (`|CreateWidget` "/Game/Blueprints/Widgets/WB_Text.WB_Text_C"))
  (bind _output_get (set `self.WB Text Ref` _returnvalue))
  (`UserWidget.AddToViewport` _output_get 0)
  (`TextBlock.SetText` (`/Game/Blueprints/Widgets/WB_Text.BuyableText` (`self.WB Text Ref`)) (`|FormatText` "Press F to get on the wagon ({wagonCost})" (`self.Wagon Cost`))))

(event `self.Box.OnComponentEndOverlap`
  (params (OverlappedComponent :type "PrimitiveComponent Object Reference") (OtherActor :type "Actor Object Reference") (OtherComp :type "PrimitiveComponent Object Reference") (OtherBodyIndex :type Integer))
  (bind _asbp_player (cast `/Game/Characters/Player/BP_Player` OtherActor))
  (set `/Game/Characters/Player/BP_Player.canSpendPoints` false _asbp_player)
  (set `self.isWagon` false)
  (`Widget.RemoveFromParent` (`self.WB Text Ref`)))

(fn `UserConstructionScript`)