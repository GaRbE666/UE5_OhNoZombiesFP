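; BP_WeaponBooster is a Pack-a-Punch style interactable that lets the player spend points to boost the equipped weapon once.
; Overlapping its trigger box stores the player and, for an unboosted weapon, shows a cost prompt widget.
; Tick polls interaction and points, then flags the weapon boosted, charges points, records its class and triggers animation and material changes on the player.
; A half-price re-boost prompt exists but is disconnected.
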(event `self.ReceiveTick`
  (params (DeltaSeconds :type "Float (single-precision)"))
  (bind _player_ref (`self.Player Ref`))
  (bind _player_ref_2 (`self.Player Ref`))
  (`/Engine/EditorBlueprintResources/StandardMacros.IsValid` (`self.Player Ref`)
    (:`Is Valid`
      ;[1 1 1] Checks
      (if (and (`/Game/Characters/Player/BP_Player.isInteracting` _player_ref) (`/Game/Characters/Player/BP_Player.canSpendPoints` _player_ref) (>= (`/Game/Characters/Player/BP_Player.Points` (`self.Player Ref`)) (`self.BoostCost`)))
        (if (and (`KismetSystemLibrary.IsValid` (`self.Player Ref`)) (not (`/Game/Weapons/Blueprints/BP_WeaponMaster.isBoosted` (`/Game/Characters/Player/BP_Player.Equipped Weapon` (`self.Player Ref`)))))
          (set `/Game/Weapons/Blueprints/BP_WeaponMaster.isBoosted` true (`/Game/Characters/Player/BP_Player.Equipped Weapon` (`self.Player Ref`)))
          (`/Game/Characters/Player/BP_Player.RemovePoints` (`self.Player Ref`) (`self.BoostCost`))
          (`Widget.RemoveFromParent` (`self.WB Text Ref`))
          (set `/Game/Characters/Player/BP_Player.canSpendPoints` false (`self.Player Ref`))
          (`KismetArrayLibrary.Array_Add` (`/Game/Characters/Player/BP_Player.WeaponsBoosted` _player_ref_2) (`GameplayStatics.GetObjectClass` (`/Game/Characters/Player/BP_Player.Equipped Weapon` _player_ref_2)))
          (`/Game/Characters/Player/BP_Player.EquipAnim` (`self.Player Ref`))
          (`/Game/Characters/Player/BP_Player.SetMaterialPAP` (`self.Player Ref`)))))))

(event `self.Box.OnComponentBeginOverlap`
  (params (OverlappedComponent :type "PrimitiveComponent Object Reference") (OtherActor :type "Actor Object Reference") (OtherComp :type "PrimitiveComponent Object Reference") (OtherBodyIndex :type Integer) (bFromSweep :type Boolean) (SweepResult :type "HitResult Structure (by ref)"))
  (bind _asbp_player (cast `/Game/Characters/Player/BP_Player` OtherActor))
  (bind _output_get (set `self.Player Ref` _asbp_player))
  (set `/Game/Characters/Player/BP_Player.canSpendPoints` true _output_get)
  ;[1 1 1] Checks
  (if (not (`/Game/Weapons/Blueprints/BP_WeaponMaster.isBoosted` (`/Game/Characters/Player/BP_Player.Equipped Weapon` (`self.Player Ref`))))
    (bind _returnvalue (`|CreateWidget` "/Game/Blueprints/Widgets/WB_Text.WB_Text_C"))
    (set `self.WB Text Ref` _returnvalue)
    (`UserWidget.AddToViewport` _returnvalue 0)
    ;[1 1 1] Boost gun
    (`TextBlock.SetText` (`/Game/Blueprints/Widgets/WB_Text.BuyableText` (`self.WB Text Ref`)) (`|FormatText` "press F to make a wonderful thing happen ({objectCost})" (`self.BoostCost`)))))

(event `self.Box.OnComponentEndOverlap`
  (params (OverlappedComponent :type "PrimitiveComponent Object Reference") (OtherActor :type "Actor Object Reference") (OtherComp :type "PrimitiveComponent Object Reference") (OtherBodyIndex :type Integer))
  (bind _asbp_player (cast `/Game/Characters/Player/BP_Player` OtherActor))
  (set `self.Player Ref` null)
  (set `/Game/Characters/Player/BP_Player.canSpendPoints` false _asbp_player)
  (`Widget.RemoveFromParent` (`self.WB Text Ref`)))

(fn `UserConstructionScript`
  (`StaticMeshComponent.SetStaticMesh` (`self.StaticMesh`) (`self.PAP Model`))
  (`SceneComponent.K2_SetRelativeTransform` (`self.Box`) (`self.Trigger Offset`) false false))