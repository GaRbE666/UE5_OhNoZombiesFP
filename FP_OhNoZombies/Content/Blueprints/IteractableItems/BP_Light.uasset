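; BP_Light is an interactable power switch that the player turns on once.
; Box overlap stores the player, enables their CanSpendPoints flag and shows a "Press F" prompt.
; Tick polls for interaction while not reloading or aiming, then sets LightIsOn, removes the prompt and disables the box.
; A DoOnce-gated timeline rotates the switch's scene component, then activates sparks and plays a power-on sound.
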(event `self.ReceiveTick`
  (params (DeltaSeconds :type "Float (single-precision)"))
  (bind _player_ref (`self.Player Ref`))
  (`/Engine/EditorBlueprintResources/StandardMacros.IsValid` (`self.Player Ref`)
    (:`Is Valid`
      ;[1 1 1] Checks
      (if (and (`/Game/Characters/Player/BP_Player.isInteracting` _player_ref) (`/Game/Characters/Player/BP_Player.canSpendPoints` _player_ref))
        (if (and (`KismetSystemLibrary.IsValid` (`self.Player Ref`)) (not (`/Game/Characters/Player/BP_Player.isReloading` (`self.Player Ref`))) (not (`/Game/Characters/Player/BP_Player.isADS` (`self.Player Ref`))))
          (set `self.LightIsOn` true)
          (set `/Game/Characters/Player/BP_Player.canSpendPoints` false (`self.Player Ref`))
          (`Widget.RemoveFromParent` (`self.WB Text Ref`))
          (`PrimitiveComponent.SetCollisionEnabled` (`self.Box`) "NoCollision")
          (`/Engine/EditorBlueprintResources/StandardMacros.DoOnce` false
            (:`Completed`
              (bind (_direction _alpha) (`Timeline|ActiveSwitchTL`)
                (:`Update`
                  (`SceneComponent.K2_SetRelativeRotation` (`self.Scene`) (`KismetMathLibrary.MakeRotator` (`KismetMathLibrary.Lerp` 25.0 -30.0 _alpha)) false false))
                (:`Finished`
                  (`ActorComponent.Activate` (`self.Sparks`) false)
                  (`GameplayStatics.SpawnSound2D` "/Game/Sounds/Richtofen_Audios/Power/powerOn_Cue.powerOn_Cue" 1.0 1.0 0.0 null))))))))))

(event `self.Box.OnComponentBeginOverlap`
  (params (OverlappedComponent :type "PrimitiveComponent Object Reference") (OtherActor :type "Actor Object Reference") (OtherComp :type "PrimitiveComponent Object Reference") (OtherBodyIndex :type Integer) (bFromSweep :type Boolean) (SweepResult :type "HitResult Structure (by ref)"))
  (bind _asbp_player (cast `/Game/Characters/Player/BP_Player` OtherActor))
  (bind _output_get (set `self.Player Ref` _asbp_player))
  (set `/Game/Characters/Player/BP_Player.canSpendPoints` true _output_get)
  (bind _returnvalue (`|CreateWidget` "/Game/Blueprints/Widgets/WB_Text.WB_Text_C"))
  (bind _output_get_2 (set `self.WB Text Ref` _returnvalue))
  (`UserWidget.AddToViewport` _output_get_2 0)
  (`TextBlock.SetText` (`/Game/Blueprints/Widgets/WB_Text.BuyableText` (`self.WB Text Ref`)) "Press F to Turn On The Power"))

(event `self.Box.OnComponentEndOverlap`
  (params (OverlappedComponent :type "PrimitiveComponent Object Reference") (OtherActor :type "Actor Object Reference") (OtherComp :type "PrimitiveComponent Object Reference") (OtherBodyIndex :type Integer))
  (bind _asbp_player (cast `/Game/Characters/Player/BP_Player` OtherActor))
  (set `self.Player Ref` null)
  (set `/Game/Characters/Player/BP_Player.canSpendPoints` false _asbp_player)
  (`/Engine/EditorBlueprintResources/StandardMacros.IsValid` (`self.WB Text Ref`)
    (:`Is Valid`
      (`Widget.RemoveFromParent` (`self.WB Text Ref`)))))

(fn `UserConstructionScript`)