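; BP_DoublePoints is a zombies-mode power-up effect actor that keeps double points active for a limited time.
; On BeginPlay it sets the flag on GM_Zombies, starts a timer and adds a WB_DoublePoints icon to the player HUD's power-up wrap box.
; Tick polls the remaining time of that dummy-function timer and destroys the actor at zero; destruction removes the widget and clears the flag.
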(event `self.ReceiveBeginPlay`
  (`self.Initialize Var`)
  (`self.Start Timer`))

(event `self.ReceiveTick`
  (params (DeltaSeconds :type "Float (single-precision)"))
  (`self.Update Timer`))

(event `self.ReceiveDestroyed`
  (`Widget.RemoveFromParent` (`self.WB DP Ref`))
  (set `/Game/Blueprints/GameModes/GM_Zombies.Double Points Is Active` false (`self.DM Zombies Ref`)))

(fn `Initialize Var`
  (bind _asbp_player (cast `/Game/Characters/Player/BP_Player` (`GameplayStatics.GetPlayerCharacter` 0)))
  (set `self.Player Ref` _asbp_player)
  (bind _asgm_zombies (cast `/Game/Blueprints/GameModes/GM_Zombies` (`GameplayStatics.GetGameMode`)))
  (bind _output_get (set `self.DM Zombies Ref` _asgm_zombies))
  (set `/Game/Blueprints/GameModes/GM_Zombies.Double Points Is Active` true _output_get))

(fn `Start Timer`
  (bind _returnvalue (`KismetSystemLibrary.K2_SetTimer` null "TimerDummy" (`self.Effect Time`)))
  (set `self.Timer Ref` _returnvalue)
  (bind _returnvalue_2 (`|CreateWidget` "/Game/Blueprints/Widgets/PowerUps/WB_DoublePoints.WB_DoublePoints_C"))
  (bind _output_get (set `self.WB DP Ref` _returnvalue_2))
  (`WrapBox.AddChildToWrapBox` (`/Game/Blueprints/Widgets/WB_MainHUD.PowerUpsWrapBox` (`/Game/Characters/Player/BP_Player.mainHUDRef` (`self.Player Ref`))) _output_get))

(fn `TimerDummy`)

(fn `Update Timer`
  (set `self.Time Remaining` (mod (/ (`KismetSystemLibrary.K2_GetTimerRemainingTimeHandle` (`self.Timer Ref`)) 1) 60))
  (if (<= (`self.Time Remaining`) 0)
    (`self.K2_DestroyActor`)))

(fn `UserConstructionScript`)