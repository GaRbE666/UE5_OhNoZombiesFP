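; BP_Pointsup is a points power-up effect actor that awards the player 500 points as soon as it begins play.
; On BeginPlay it caches the player, adds a WB_PointsUp widget to the HUD's power-up wrap box and starts an EffectTime timer on an empty dummy function.
; Tick polls that timer's remaining time and destroys the actor at zero, which removes the widget.
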(event `self.ReceiveBeginPlay`
  (`self.Initialize Var`)
  (`self.Start Timer`))

(event `self.ReceiveTick`
  (params (DeltaSeconds :type "Float (single-precision)"))
  (`self.Update Timer`))

(event `self.ReceiveDestroyed`
  (`Widget.RemoveFromParent` (`self.WB PU Ref`)))

(fn `Initialize Var`
  (bind _asbp_player (cast `/Game/Characters/Player/BP_Player` (`GameplayStatics.GetPlayerCharacter` 0)))
  (set `self.Player Ref` _asbp_player))

(fn `Start Timer`
  (bind _returnvalue (`KismetSystemLibrary.K2_SetTimer` null "TimerDummy" (`self.Effect Time`)))
  (set `self.Timer Ref` _returnvalue)
  (bind _returnvalue_2 (`|CreateWidget` "/Game/Blueprints/Widgets/PowerUps/WB_PointsUp.WB_PointsUp_C"))
  (bind _output_get (set `self.WB PU Ref` _returnvalue_2))
  (`WrapBox.AddChildToWrapBox` (`/Game/Blueprints/Widgets/WB_MainHUD.PowerUpsWrapBox` (`/Game/Characters/Player/BP_Player.mainHUDRef` (`self.Player Ref`))) _output_get)
  (`/Game/Characters/Player/BP_Player.AddPoints` (`self.Player Ref`) 500))

(fn `TimerDummy`)

(fn `Update Timer`
  (set `self.Time Remaining` (mod (/ (`KismetSystemLibrary.K2_GetTimerRemainingTimeHandle` (`self.Timer Ref`)) 1) 60))
  (if (<= (`self.Time Remaining`) 0)
    (`self.K2_DestroyActor`)))

(fn `UserConstructionScript`)