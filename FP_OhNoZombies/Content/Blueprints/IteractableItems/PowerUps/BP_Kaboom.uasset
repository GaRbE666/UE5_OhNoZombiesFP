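; BP_Kaboom is a power-up actor that kills every living zombie once when it spawns.
; On BeginPlay it adds a Kaboom widget to the player's HUD, sets KaboomIsActive on GM_Zombies and deals massive damage to each living BP_AI_Zombie.
; An empty-function timer serves as the effect countdown, polled on Tick to destroy the actor.
; Destruction removes the widget and clears the game mode flag.
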(event `self.ReceiveBeginPlay`
  (`self.Initialize Var`)
  (`self.Start Timer`))

(event `self.ReceiveTick`
  (params (DeltaSeconds :type "Float (single-precision)"))
  (`self.Update Timer`))

(event `self.ReceiveDestroyed`
  (`Widget.RemoveFromParent` (`self.WB KB Ref`))
  (set `/Game/Blueprints/GameModes/GM_Zombies.Kaboom Is Active` false (`self.GM Zombies Ref`)))

(fn `Initialize Var`
  (bind _asbp_player (cast `/Game/Characters/Player/BP_Player` (`GameplayStatics.GetPlayerCharacter` 0)))
  (set `self.Player Ref` _asbp_player))

(fn `Start Timer`
  (bind _returnvalue (`KismetSystemLibrary.K2_SetTimer` null "TimerDummy" (`self.Effect Time`)))
  (set `self.Timer Ref` _returnvalue)
  (bind _returnvalue_2 (`|CreateWidget` "/Game/Blueprints/Widgets/PowerUps/WB_Kaboom.WB_Kaboom_C"))
  (bind _output_get (set `self.WB KB Ref` _returnvalue_2))
  (`WrapBox.AddChildToWrapBox` (`/Game/Blueprints/Widgets/WB_MainHUD.PowerUpsWrapBox` (`/Game/Characters/Player/BP_Player.mainHUDRef` (`self.Player Ref`))) _output_get)
  (bind _asgm_zombies (cast `/Game/Blueprints/GameModes/GM_Zombies` (`GameplayStatics.GetGameMode`)))
  (bind _output_get_2 (set `self.GM Zombies Ref` _asgm_zombies))
  (set `/Game/Blueprints/GameModes/GM_Zombies.Kaboom Is Active` true _output_get_2)
  ;[1 1 1] Kill All zombies
  (bind _outactors (`GameplayStatics.GetAllActorsOfClass` "/Game/Characters/Zombie/Blueprints/BP_AI_Zombie.BP_AI_Zombie_C"))
  (for _array_element _outactors
    (if (not (<= (`/Game/Blueprints/Components/BPC_Health.Current Health` (`/Game/Characters/Zombie/Blueprints/BP_AI_Zombie.BPC_Health` _array_element)) 0.0))
      (`/Game/Characters/Zombie/Blueprints/BP_AI_Zombie.TakeDamage` _array_element 999999.0 "None" (0.0 0.0 0.0)))))

(fn `TimerDummy`)

(fn `Update Timer`
  (set `self.Time Remaining` (mod (/ (`KismetSystemLibrary.K2_GetTimerRemainingTimeHandle` (`self.Timer Ref`)) 1) 60))
  (if (<= (`self.Time Remaining`) 0)
    (`self.K2_DestroyActor`)))

(fn `UserConstructionScript`)