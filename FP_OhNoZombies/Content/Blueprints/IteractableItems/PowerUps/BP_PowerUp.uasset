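; BP_PowerUp is a zombies-mode pickup that activates one of four power-ups when the player overlaps it, or expires if left uncollected.
; On overlap it disables collision and uses PowerUpType to spawn the matching effect actor.
; Double Points replaces existing instances, while Insta Kill, Kaboom and Points Up spawn, and destroy the pickup, only when none exist.
; Tick polls a timer's remaining time to handle expiry.
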(event `self.ReceiveBeginPlay`
  (`self.StartTimerToDestroy`)
  (set `self.Item Collected` false))

(event `self.ReceiveTick`
  (params (DeltaSeconds :type "Float (single-precision)"))
  (if (not (`self.Item Collected`))
    (`self.UpdateDestroyTimer`)))

(event `self.Box.OnComponentBeginOverlap`
  (params (OverlappedComponent :type "PrimitiveComponent Object Reference") (OtherActor :type "Actor Object Reference") (OtherComp :type "PrimitiveComponent Object Reference") (OtherBodyIndex :type Integer) (bFromSweep :type Boolean) (SweepResult :type "HitResult Structure (by ref)"))
  (bind _asbp_player (cast `/Game/Characters/Player/BP_Player` OtherActor))
  (set `self.Player Ref` _asbp_player)
  (set `self.Item Collected` true)
  (`StaticMeshComponent.SetStaticMesh` (`self.StaticMesh`) null)
  (`PrimitiveComponent.SetCollisionEnabled` (`self.Box`) "NoCollision")
  (switch `/Game/Blueprints/IteractableItems/PowerUps/PowerUpEnum` (`self.PowerUp Type`)
    (:`NewEnumerator0`
      ;[1 1 1] Insta Kill Spawn
      (bind _outactors (`GameplayStatics.GetAllActorsOfClass` "/Game/Blueprints/IteractableItems/PowerUps/BP_InstaKill.BP_InstaKill_C"))
      (if (== (`KismetArrayLibrary.Array_Length` _outactors) 0)
        (`|SpawnActorFromClass` "/Game/Blueprints/IteractableItems/PowerUps/BP_InstaKill.BP_InstaKill_C" (`self.GetTransform`) "Undefined" "OverrideRootScale" null null)
        (`self.K2_DestroyActor`)))
    (:`NewEnumerator1`
      ;[1 1 1] Kaboom Spawn
      (bind _outactors_2 (`GameplayStatics.GetAllActorsOfClass` "/Game/Blueprints/IteractableItems/PowerUps/BP_Kaboom.BP_Kaboom_C"))
      (if (== (`KismetArrayLibrary.Array_Length` _outactors_2) 0)
        (`|SpawnActorFromClass` "/Game/Blueprints/IteractableItems/PowerUps/BP_Kaboom.BP_Kaboom_C" (`self.GetTransform`) "Undefined" "OverrideRootScale" null null)
        (`self.K2_DestroyActor`)))
    (:`NewEnumerator2`
      ;[1 1 1] Double Points Spawn
      (bind _outactors_3 (`GameplayStatics.GetAllActorsOfClass` "/Game/Blueprints/IteractableItems/PowerUps/BP_DoublePoints.BP_DoublePoints_C"))
      (if (not (== (`KismetArrayLibrary.Array_Length` _outactors_3) 0))
        (for _array_element _outactors_3
          (`self.K2_DestroyActor` _array_element)))
      (`|SpawnActorFromClass` "/Game/Blueprints/IteractableItems/PowerUps/BP_DoublePoints.BP_DoublePoints_C" (`self.GetTransform`) "Undefined" "OverrideRootScale" null null)
      (`self.K2_DestroyActor`))
    (:`NewEnumerator4`
      ;[1 1 1] Points Up Spawn
      (bind _outactors_4 (`GameplayStatics.GetAllActorsOfClass` "/Game/Blueprints/IteractableItems/PowerUps/BP_Pointsup.BP_Pointsup_C"))
      (if (== (`KismetArrayLibrary.Array_Length` _outactors_4) 0)
        (`|SpawnActorFromClass` "/Game/Blueprints/IteractableItems/PowerUps/BP_Pointsup.BP_Pointsup_C" (`self.GetTransform`) "Undefined" "OverrideRootScale" null null)
        (`self.K2_DestroyActor`)))))

(fn `StartTimerToDestroy`
  (bind _returnvalue (`KismetSystemLibrary.K2_SetTimer` null "TimerEnd" (`self.Time To Destroy`)))
  (set `self.Timer To Destroy Ref` _returnvalue))

(fn `TimerEnd`)

(fn `UpdateDestroyTimer`
  (set `self.Destroy Seconds Left` (mod (/ (`KismetSystemLibrary.K2_GetTimerRemainingTimeHandle` (`self.Timer To Destroy Ref`)) 1) 60))
  (if (<= (`self.Destroy Seconds Left`) 0)
    (`self.K2_DestroyActor`)))

(fn `UserConstructionScript`)