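; BP_Impulse is an interactable trigger volume that launches the player after a short charge-up.
; Entering the Box starts a two-second timer that applies ImpulseForce to the player's CharacterMovement as a velocity-change impulse.
; Leaving the Box clears the timer, cancelling the launch.
; While the timer is active, Tick plays a world camera shake at the player's location every frame.
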(event `self.ReceiveTick`
  (params (DeltaSeconds :type "Float (single-precision)"))
  (`self.PlayerCameraShake`))

(event `self.Box.OnComponentBeginOverlap`
  (params (OverlappedComponent :type "PrimitiveComponent Object Reference") (OtherActor :type "Actor Object Reference") (OtherComp :type "PrimitiveComponent Object Reference") (OtherBodyIndex :type Integer) (bFromSweep :type Boolean) (SweepResult :type "HitResult Structure (by ref)"))
  (bind _asbp_player (cast `/Game/Characters/Player/BP_Player` OtherActor))
  (set `self.Player Ref` _asbp_player)
  (bind _returnvalue (`KismetSystemLibrary.K2_SetTimer` null "ImpulsePlayer" 2.0))
  (set `self.Impulse Timer` _returnvalue))

(event `self.Box.OnComponentEndOverlap`
  (params (OverlappedComponent :type "PrimitiveComponent Object Reference") (OtherActor :type "Actor Object Reference") (OtherComp :type "PrimitiveComponent Object Reference") (OtherBodyIndex :type Integer))
  (cast `/Game/Characters/Player/BP_Player` OtherActor)
  (`KismetSystemLibrary.K2_ClearAndInvalidateTimerHandle` (`self.Impulse Timer`)))

(event `ImpulsePlayer`
  (`CharacterMovementComponent.AddImpulse` (`Character.CharacterMovement` (`self.Player Ref`)) (`self.Impulse Force`) true))

(fn `PlayerCameraShake`
  (bind _player_ref (`self.Player Ref`))
  (if (`KismetSystemLibrary.K2_IsTimerActiveHandle` (`self.Impulse Timer`))
    (`/Engine/EditorBlueprintResources/StandardMacros.IsValid` _player_ref
      (:`Is Valid`
        (`GameplayStatics.PlayWorldCameraShake` "/Game/Blueprints/BP_CameraShake.BP_CameraShake_C" (`self.K2_GetActorLocation` _player_ref) 0.0 1000.0)))))

(fn `UserConstructionScript`)