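; BP_Statue is an Easter egg step actor for the zombies mode: a statue holding a glow stick the player can take.
; On BeginPlay a timeline raises the statue between fixed world heights and flags it as in the map when finished.
; Tick polls the GM_Zombies Easter egg stage and player interaction inside the box overlap.
; Pickup destroys the stick, plays a sound, flags the player, advances the stage and reverses the timeline.
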(event `self.ReceiveBeginPlay`
  (bind _statue (`self.Statue`))
  (bind (_returnvalue_x _returnvalue_y) (`KismetMathLibrary.BreakVector` (`SceneComponent.K2_GetComponentLocation` _statue)))
  (bind _asbp_player (cast `/Game/Characters/Player/BP_Player` (`GameplayStatics.GetPlayerCharacter` 0)))
  (set `self.Player Ref` _asbp_player)
  (bind _asgm_zombies (cast `/Game/Blueprints/GameModes/GM_Zombies` (`GameplayStatics.GetGameMode`)))
  (set `self.GM Zombie Ref` _asgm_zombies)
  (bind (_direction _alpha) (`Timeline|StatueUpTL` :!label _label)
    (:`Update`
      (`SceneComponent.K2_SetWorldLocation` _statue (`KismetMathLibrary.MakeVector` _returnvalue_x _returnvalue_y (`KismetMathLibrary.Lerp` 9665.0 9990.0 _alpha)) false false))
    (:`Finished`
      (switch `ETimelineDirection` _direction
        (:`Forward`
          (set `self.Statue Is In Map` true))))))

(event `self.ReceiveTick`
  (params (DeltaSeconds :type "Float (single-precision)"))
  (if (and (`|EnumEquality` (`/Game/Blueprints/GameModes/GM_Zombies.EEEnum` (`self.GM Zombie Ref`)) "NewEnumerator2") (`self.Statue Is In Map`))
    (if (and (`/Game/Characters/Player/BP_Player.isInteracting` (`self.Player Ref`)) (`self.Can Grab Stick Bar`))
      (`PrimitiveComponent.SetCollisionEnabled` (`self.Box`) "NoCollision")
      (`ActorComponent.K2_DestroyComponent` (`self.Stick`))
      (`GameplayStatics.SpawnSound2D` "/Game/Sounds/SongParts/PickPart_Cue.PickPart_Cue" 1.0 1.0 0.0 null)
      (set `/Game/Characters/Player/BP_Player.I Have Glow Stick` true (`self.Player Ref`))
      (set `self.Statue Is In Map` false)
      (set `/Game/Blueprints/GameModes/GM_Zombies.EEEnum` "NewEnumerator3" (`self.GM Zombie Ref`))
      (goto _label :!via `Reverse`))))

(event `self.Box.OnComponentBeginOverlap`
  (params (OverlappedComponent :type "PrimitiveComponent Object Reference") (OtherActor :type "Actor Object Reference") (OtherComp :type "PrimitiveComponent Object Reference") (OtherBodyIndex :type Integer) (bFromSweep :type Boolean) (SweepResult :type "HitResult Structure (by ref)"))
  (cast `/Game/Characters/Player/BP_Player` OtherActor)
  (set `self.Can Grab Stick Bar` true))

(event `self.Box.OnComponentEndOverlap`
  (params (OverlappedComponent :type "PrimitiveComponent Object Reference") (OtherActor :type "Actor Object Reference") (OtherComp :type "PrimitiveComponent Object Reference") (OtherBodyIndex :type Integer))
  (cast `/Game/Characters/Player/BP_Player` OtherActor)
  (set `self.Can Grab Stick Bar` false))

(fn `UserConstructionScript`)