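; BP_JailStick is an interactable wooden-cage prop where the player places a glow stick as one step of the Zombies mode Easter egg.
; Box overlaps track whether the player is in range, while Tick checks for the glow stick, interact input and the required EEEnum stage in GM_Zombies.
; When all hold, a DoOnce swaps the cage mesh, reveals the stick, advances the stage and plays a pickup sound.
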(event `self.ReceiveBeginPlay`
  (bind _asbp_player (cast `/Game/Characters/Player/BP_Player` (`GameplayStatics.GetPlayerCharacter` 0)))
  (set `self.Player Ref` _asbp_player)
  (bind _asgm_zombies (cast `/Game/Blueprints/GameModes/GM_Zombies` (`GameplayStatics.GetGameMode`)))
  (set `self.GM Zombie Ref` _asgm_zombies)
  (`SceneComponent.SetVisibility` (`self.Stick`) false false)
  (`StaticMeshComponent.SetStaticMesh` (`self.StaticMesh`) "/Game/ModularLostRuinKit/Models/Structure/WFoliage/SM_Wood_Cage_2X3_Fol.SM_Wood_Cage_2X3_Fol")
  (`ActorComponent.SetActive` (`self.Box`) false false))

(event `self.ReceiveTick`
  (params (DeltaSeconds :type "Float (single-precision)"))
  (if (and (`/Game/Characters/Player/BP_Player.I Have Glow Stick` (`self.Player Ref`)) (`|EnumEquality` (`/Game/Blueprints/GameModes/GM_Zombies.EEEnum` (`self.GM Zombie Ref`)) "NewEnumerator3") (`/Game/Characters/Player/BP_Player.isInteracting` (`self.Player Ref`)) (`self.Can Put Stick`))
    (`/Engine/EditorBlueprintResources/StandardMacros.DoOnce` false
      (:`Completed`
        (`StaticMeshComponent.SetStaticMesh` (`self.StaticMesh`) "/Game/ModularLostRuinKit/Models/Structure/SM_Wood_Cage_2X2.SM_Wood_Cage_2X2")
        (`SceneComponent.SetVisibility` (`self.Stick`) true false)
        (set `/Game/Blueprints/GameModes/GM_Zombies.EEEnum` "NewEnumerator4" (`self.GM Zombie Ref`))
        (`GameplayStatics.SpawnSound2D` "/Game/Sounds/SongParts/PickPart_Cue.PickPart_Cue" 1.0 1.0 0.0 null)))))

(event `self.Box.OnComponentBeginOverlap`
  (params (OverlappedComponent :type "PrimitiveComponent Object Reference") (OtherActor :type "Actor Object Reference") (OtherComp :type "PrimitiveComponent Object Reference") (OtherBodyIndex :type Integer) (bFromSweep :type Boolean) (SweepResult :type "HitResult Structure (by ref)"))
  (cast `/Game/Characters/Player/BP_Player` OtherActor)
  (set `self.Can Put Stick` true))

(event `self.Box.OnComponentEndOverlap`
  (params (OverlappedComponent :type "PrimitiveComponent Object Reference") (OtherActor :type "Actor Object Reference") (OtherComp :type "PrimitiveComponent Object Reference") (OtherBodyIndex :type Integer))
  (cast `/Game/Characters/Player/BP_Player` OtherActor)
  (set `self.Can Put Stick` false))

(fn `UserConstructionScript`)