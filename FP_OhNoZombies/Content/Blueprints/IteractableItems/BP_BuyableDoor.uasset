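; Buyable door that a player opens with points, clearing the way and linked to zombie spawner activation.
; Box overlap shows a price prompt, and Tick polls for interact and enough points, sometimes playing a no-money sound otherwise.
; A timeline lifts the mesh, with event tracks removing points, collision and text and starting two debris timelines.
; On finish it destroys itself and listed debris; its spawner loop only spawns for invalid SpawnPoints entries.
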(event `self.ReceiveTick`
  (params (DeltaSeconds :type "Float (single-precision)"))
  (bind _playerref (`self.PlayerRef`))
  (bind _buyablemesh (`self.BuyableMesh`))
  (bind _buyablemesh1 (`self.BuyableMesh1`))
  (bind _buyablemesh2 (`self.BuyableMesh2`))
  (bind (_relativelocation_x _relativelocation_y) (`KismetMathLibrary.BreakVector` (`SceneComponent.RelativeLocation` _buyablemesh1)))
  (bind (_relativelocation_x_2 _relativelocation_y_2) (`KismetMathLibrary.BreakVector` (`SceneComponent.RelativeLocation` _buyablemesh)))
  (bind (_relativelocation_x_3 _relativelocation_y_3) (`KismetMathLibrary.BreakVector` (`SceneComponent.RelativeLocation` _buyablemesh2)))
  (`/Engine/EditorBlueprintResources/StandardMacros.IsValid` (`self.PlayerRef`)
    (:`Is Valid`
      ;[1 1 1] Checks
      (if (and (`/Game/Characters/Player/BP_Player.isInteracting` _playerref) (`/Game/Characters/Player/BP_Player.canSpendPoints` _playerref))
        (if (>= (`/Game/Characters/Player/BP_Player.Points` (`self.PlayerRef`)) (`self.Object Cost`))
          (if (`KismetSystemLibrary.IsValid` (`self.PlayerRef`))
            (`|ExecutionSequence`
              (:`then_0`
                (`/Engine/EditorBlueprintResources/StandardMacros.DoOnce` false
                  (:`Completed`
                    (`GameplayStatics.SpawnSound2D` (`self.Audio`) 1.0 1.0 0.0 null))))
              (:`then_1`
                (bind (_direction _alpha) (`Timeline|OpenDoorTL`)
                  (:`Update`
                    ;[1 1 1] Update Mesh
                    (`SceneComponent.K2_SetRelativeLocation` _buyablemesh (`KismetMathLibrary.MakeVector` _relativelocation_x_2 _relativelocation_y_2 (`KismetMathLibrary.Lerp` 0.0 1000.0 _alpha)) false false))
                  (:`Finished`
                    ;[1 1 1] Finish Anim
                    (`self.K2_DestroyActor`)
                    (`self.Activate Sapwns`)
                    (`self.Destroy Debris`))
                  (:`DisableCollision`
                    ;[1 1 1] Manage Collision
                    (`PrimitiveComponent.SetCollisionEnabled` (`self.BuyableMesh`) "NoCollision")
                    (`ActorComponent.K2_DestroyComponent` (`self.Box`))
                    (`self.DisableMeshCollision`))
                  (:`DisableText`
                    ;[1 1 1] Remove Text
                    (`Widget.RemoveFromParent` (`self.WBDoorTextRef`)))
                  (:`RemovePoints`
                    ;[1 1 1] Remove Points
                    (`/Game/Characters/Player/BP_Player.RemovePoints` (`self.PlayerRef`) (`self.Object Cost`)))
                  (:`ActiveDebris2`
                    ;[1 1 1] Debris 2 Anim
                    (bind (_direction_2 _alpha_2) (`Timeline|Debris2AnimTL`)
                      (:`Update`
                        (`SceneComponent.K2_SetRelativeLocation` _buyablemesh1 (`KismetMathLibrary.MakeVector` _relativelocation_x _relativelocation_y (`KismetMathLibrary.Lerp` 105.0 1000.0 _alpha_2)) false false))))
                  (:`ActiveDebris3`
                    ;[1 1 1] Debris 3 Anim
                    (bind (_direction_3 _alpha_3) (`Timeline|Debris3AnimTL`)
                      (:`Update`
                        (`SceneComponent.K2_SetRelativeLocation` _buyablemesh2 (`KismetMathLibrary.MakeVector` _relativelocation_x_3 _relativelocation_y_3 (`KismetMathLibrary.Lerp` 0.0 1000.0 _alpha_3)) false false))))))))
          (else
            ;[1 1 1] Sound No money
            (if (> (`KismetMathLibrary.RandomFloatInRange` 0.0 1.0) 0.5)
              (`/Game/Characters/Player/BP_Player.PlaySound` (`self.PlayerRef`) "/Game/Sounds/Richtofen_Audios/NoMoney/NoMoney_Cue.NoMoney_Cue"))))))))

(event `self.Box.OnComponentBeginOverlap`
  (params (OverlappedComponent :type "PrimitiveComponent Object Reference") (OtherActor :type "Actor Object Reference") (OtherComp :type "PrimitiveComponent Object Reference") (OtherBodyIndex :type Integer) (bFromSweep :type Boolean) (SweepResult :type "HitResult Structure (by ref)"))
  (bind _asbp_player (cast `/Game/Characters/Player/BP_Player` OtherActor))
  (set `self.PlayerRef` _asbp_player)
  (set `/Game/Characters/Player/BP_Player.canSpendPoints` true _asbp_player)
  (bind _returnvalue (`|CreateWidget` "/Game/Blueprints/Widgets/WB_Text.WB_Text_C"))
  (set `self.WBDoorTextRef` _returnvalue)
  (`UserWidget.AddToViewport` _returnvalue 0)
  ;[1 1 1] Door Text
  (`TextBlock.SetText` (`/Game/Blueprints/Widgets/WB_Text.BuyableText` (`self.WBDoorTextRef`)) (`|FormatText` "Press F to open door ({doorCost})" (`self.Object Cost`))))

(event `self.Box.OnComponentEndOverlap`
  (params (OverlappedComponent :type "PrimitiveComponent Object Reference") (OtherActor :type "Actor Object Reference") (OtherComp :type "PrimitiveComponent Object Reference") (OtherBodyIndex :type Integer))
  (bind _asbp_player (cast `/Game/Characters/Player/BP_Player` OtherActor))
  (set `self.PlayerRef` null)
  (set `/Game/Characters/Player/BP_Player.canSpendPoints` false _asbp_player)
  (`Widget.RemoveFromParent` (`self.WBDoorTextRef`)))

(fn `Activate Sapwns`
  (for _array_element (`self.Spawn Points`)
    (`/Engine/EditorBlueprintResources/StandardMacros.IsValid` _array_element
      (:`Is Not Valid`
        (`|SpawnActorFromClass` "/Game/Blueprints/BP_ZombieSpawner.BP_ZombieSpawner_C" (`self.GetTransform` _array_element) "Undefined" "OverrideRootScale" null null)))))

(fn `Destroy Debris`
  (if (`KismetArrayLibrary.Array_IsNotEmpty` (`self.Debris`))
    (for _array_element (`self.Debris`)
      (`/Engine/EditorBlueprintResources/StandardMacros.IsValid` _array_element
        (:`Is Valid`
          (`self.K2_DestroyActor` _array_element))))))

(fn `DisableMeshCollision`
  (`PrimitiveComponent.SetCollisionEnabled` (`self.BuyableMesh`) "NoCollision")
  (`PrimitiveComponent.SetCollisionEnabled` (`self.BuyableMesh1`) "NoCollision")
  (`PrimitiveComponent.SetCollisionEnabled` (`self.BuyableMesh2`) "NoCollision"))

(fn `UserConstructionScript`
  (`SceneComponent.K2_SetRelativeTransform` (`self.Box`) (`self.Collider Transform`) false false))