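; BP_BuyableGun is a wall-buy style pickup that sells a configurable weapon, or ammo for it, for player points.
; Box overlap stores the player, enables spending and shows a price prompt widget.
; Tick polls interaction and checks points against the gun cost, even for ammo, which refills only the equipped matching weapon.
; New purchases replace the held weapon when two are carried, then equip, with a timeline sliding the mesh.
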(event `self.ReceiveTick`
  (params (DeltaSeconds :type "Float (single-precision)"))
  (bind _playerref (`self.PlayerRef`))
  (`/Engine/EditorBlueprintResources/StandardMacros.IsValid` (`self.PlayerRef`)
    (:`Is Valid`
      ;[1 1 1] Checks
      (if (and (`/Game/Characters/Player/BP_Player.isInteracting` _playerref) (`/Game/Characters/Player/BP_Player.canSpendPoints` _playerref) (>= (`/Game/Characters/Player/BP_Player.Points` (`self.PlayerRef`)) (`self.Object Cost`)))
        (if (`KismetSystemLibrary.IsValid` (`self.PlayerRef`))
          ;[1 1 1] Weapon
          (if (`self.Check if I Have Weapon`)
            ;;[1 1 1] Add Ammo
            (if (== (`self.Get Weapon Class`) (`self.Weapon Class`))
              (`/Game/Characters/Player/BP_Player.Max Ammo Current Weapon` (`self.PlayerRef`) (`self.Weapon Class`))
              (`/Game/Characters/Player/BP_Player.RemovePoints` (`self.PlayerRef`) (`self.Ammo Cost`))
              (set `/Game/Characters/Player/BP_Player.canSpendPoints` false (`self.PlayerRef`))
              (`GameplayStatics.SpawnSound2D` "/Game/Sounds/BuySound_Cue.BuySound_Cue" 1.0 1.0 0.0 null :!label _label)
              (goto _label_2 :!via `Reset`)
              (else
                (set `/Game/Characters/Player/BP_Player.canSpendPoints` false (`self.PlayerRef`))))
            (else
              (`/Engine/EditorBlueprintResources/StandardMacros.DoOnce` false :!label _label_2
                (:`Completed`
                  (if (not (< (`KismetArrayLibrary.Array_Length` (`/Game/Characters/Player/BP_Player.WeaponsEquiped` (`self.PlayerRef`))) 2))
                    (`self.Replace Current Weapon`))
                  ;;[1 1 1] Add New Wepon
                  (`self.Add Weapon To Player`)
                  (`/Game/Characters/Player/BP_Player.Equip Weapon` (`self.PlayerRef`) (`self.Weapon Class`))
                  (set `/Game/Characters/Player/BP_Player.WeaponIndex` (`KismetArrayLibrary.Array_Find` (`/Game/Characters/Player/BP_Player.WeaponsEquiped` (`self.PlayerRef`)) (`self.Weapon Class`)) (`self.PlayerRef`))
                  (set `/Game/Characters/Player/BP_Player.canSpendPoints` false (`self.PlayerRef`))
                  (bind (_direction _alpha) (`Timeline|PurchasedWeaponTL`)
                    (:`Update`
                      (`SceneComponent.K2_SetRelativeLocation` (`self.StaticMesh`) (`KismetMathLibrary.MakeVector` 0.0 (`KismetMathLibrary.Lerp` 0.0 10.0 _alpha)) false false))
                    (:`Finished`
                      (goto _label_2 :!via `Reset`))
                    (:`Sound`
                      (goto _label))))))))))))

(event `self.Box.OnComponentBeginOverlap`
  (params (OverlappedComponent :type "PrimitiveComponent Object Reference") (OtherActor :type "Actor Object Reference") (OtherComp :type "PrimitiveComponent Object Reference") (OtherBodyIndex :type Integer) (bFromSweep :type Boolean) (SweepResult :type "HitResult Structure (by ref)"))
  (bind _asbp_player (cast `/Game/Characters/Player/BP_Player` OtherActor))
  (set `self.PlayerRef` _asbp_player)
  (set `/Game/Characters/Player/BP_Player.canSpendPoints` true _asbp_player)
  (bind _returnvalue (`|CreateWidget` "/Game/Blueprints/Widgets/WB_Text.WB_Text_C"))
  (set `self.WB Text Ref` _returnvalue)
  (`UserWidget.AddToViewport` _returnvalue 0)
  ;[1 1 1] Check 1
  (if (`self.Check if I Have Weapon`)
    (if (== (`self.Get Weapon Class`) (`self.Weapon Class`))
      ;[1 1 1] Ammo Text
      (`TextBlock.SetText` (`/Game/Blueprints/Widgets/WB_Text.BuyableText` (`self.WB Text Ref`)) (`|FormatText` "Press F to buy ammo ({objectCost})" (`self.Ammo Cost`))))
    (else
      ;[1 1 1] Buy Gun Text
      (`TextBlock.SetText` (`/Game/Blueprints/Widgets/WB_Text.BuyableText` (`self.WB Text Ref`)) (`|FormatText` "Press F to buy {WeaponName} ({objectCost})" (`self.Weapon Name`) (`self.Object Cost`))))))

(event `self.Box.OnComponentEndOverlap`
  (params (OverlappedComponent :type "PrimitiveComponent Object Reference") (OtherActor :type "Actor Object Reference") (OtherComp :type "PrimitiveComponent Object Reference") (OtherBodyIndex :type Integer))
  (bind _asbp_player (cast `/Game/Characters/Player/BP_Player` OtherActor))
  (set `self.PlayerRef` null)
  (set `/Game/Characters/Player/BP_Player.canSpendPoints` false _asbp_player)
  (`Widget.RemoveFromParent` (`self.WB Text Ref`)))

(fn `Add Weapon To Player`
  (`KismetArrayLibrary.Array_Add` (`/Game/Characters/Player/BP_Player.WeaponsEquiped` (`self.PlayerRef`)) (`self.Weapon Class`))
  (`Widget.RemoveFromParent` (`self.WB Text Ref`))
  (`/Game/Characters/Player/BP_Player.RemovePoints` (`self.PlayerRef`) (`self.Object Cost`)))

(fn `Check if I Have Weapon`
  (returns (ReturnValue :type Boolean))
  (bind _weaponsequiped (`/Game/Characters/Player/BP_Player.WeaponsEquiped` (`self.PlayerRef`)))
  (return (`KismetArrayLibrary.Array_IsValidIndex` _weaponsequiped (`KismetArrayLibrary.Array_Find` _weaponsequiped (`self.Weapon Class`)))))

(fn `Get Weapon Class`
  (returns (ReturnValue :type "/Game/Weapons/Blueprints/BP_WeaponMaster Class Reference"))
  (return (`GameplayStatics.GetObjectClass` (`/Game/Characters/Player/BP_Player.Equipped Weapon` (`self.PlayerRef`)))))

(fn `Replace Current Weapon`
  (bind _playerref (`self.PlayerRef`))
  (`KismetArrayLibrary.Array_RemoveItem` (`/Game/Characters/Player/BP_Player.WeaponsEquiped` _playerref) (`GameplayStatics.GetObjectClass` (`/Game/Characters/Player/BP_Player.Equipped Weapon` _playerref))))

(fn `UserConstructionScript`
  (`StaticMeshComponent.SetStaticMesh` (`self.StaticMesh`) (`self.mesh`))
  (`TextRenderComponent.K2_SetText` (`self.TextRender`) (`KismetTextLibrary.Conv_StringToText` (`self.Weapon Name`))))