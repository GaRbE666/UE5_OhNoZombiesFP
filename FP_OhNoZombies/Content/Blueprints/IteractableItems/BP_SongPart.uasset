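; BP_SongPart is an interactable collectible for a song easter egg in the Zombies mode, playing an ambient sound until picked up.
; Box overlaps track the player, and Tick polls IsInteracting to stop the ambience, increment GM_Zombies.SongCount once and play that count's voice cue.
; The first two pickups disable box collision.
; With no player in range, each instance plays the completion cue after a delay once the count reaches three.
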(event `self.ReceiveBeginPlay`
  (bind _returnvalue (`GameplayStatics.SpawnSoundAtLocation` (`self.Ambient Sound`) (`SceneComponent.K2_GetComponentLocation` (`self.StaticMesh`)) (struct) (`self.Volume Ambien Sound`) 1.0 0.0 "/Game/Sounds/SongParts/NewSoundAttenuation.NewSoundAttenuation" null false))
  (set `self.Ambien Audio` _returnvalue))

(event `self.ReceiveTick`
  (params (DeltaSeconds :type "Float (single-precision)"))
  (bind _player_ref (`self.Player Ref`))
  (`/Engine/EditorBlueprintResources/StandardMacros.IsValid` (`self.Player Ref`)
    (:`Is Valid`
      (if (`/Game/Characters/Player/BP_Player.isInteracting` (`self.Player Ref`))
        (`/Engine/EditorBlueprintResources/StandardMacros.DoOnce` false
          (:`Completed`
            (`AudioComponent.Stop` (`self.Ambien Audio`))
            (`GameplayStatics.PlaySound2D` "/Game/Sounds/SongParts/PickPart_Cue.PickPart_Cue" 1.0 1.0 0.0 null null)
            (bind _asgm_zombies (cast `/Game/Blueprints/GameModes/GM_Zombies` (`GameplayStatics.GetGameMode`)))
            (bind _songcount (`/Game/Blueprints/GameModes/GM_Zombies.SongCount` _asgm_zombies))
            (`/Engine/EditorBlueprintResources/StandardMacros.IncrementInt` _songcount
              (:`  `
                (switch `int` _songcount
                  (:`1`
                    (`/Game/Characters/Player/BP_Player.PlaySound` _player_ref "/Game/Sounds/Richtofen_Audios/Song/Part1_Cue.Part1_Cue")
                    (`PrimitiveComponent.SetCollisionEnabled` (`self.Box`) "NoCollision" :!label _label))
                  (:`2`
                    (`/Game/Characters/Player/BP_Player.PlaySound` _player_ref "/Game/Sounds/Richtofen_Audios/Song/Part2_Cue.Part2_Cue")
                    (goto _label))
                  (:`3`
                    (`/Game/Characters/Player/BP_Player.PlaySound` _player_ref "/Game/Sounds/Richtofen_Audios/Song/Part3_Cue.Part3_Cue")))))))))
    (:`Is Not Valid`
      (bind _asgm_zombies_2 (cast `/Game/Blueprints/GameModes/GM_Zombies` (`GameplayStatics.GetGameMode`)))
      (if (== (`/Game/Blueprints/GameModes/GM_Zombies.SongCount` _asgm_zombies_2) 3)
        (`/Engine/EditorBlueprintResources/StandardMacros.DoOnce` false
          (:`Completed`
            (`KismetSystemLibrary.Delay` 5.0)
            (bind _asbp_player (cast `/Game/Characters/Player/BP_Player` (`GameplayStatics.GetPlayerCharacter` 0)))
            (`/Game/Characters/Player/BP_Player.PlaySound` _asbp_player "/Game/Sounds/Richtofen_Audios/Song/SongCompleted_Cue.SongCompleted_Cue")))))))

(event `self.Box.OnComponentBeginOverlap`
  (params (OverlappedComponent :type "PrimitiveComponent Object Reference") (OtherActor :type "Actor Object Reference") (OtherComp :type "PrimitiveComponent Object Reference") (OtherBodyIndex :type Integer) (bFromSweep :type Boolean) (SweepResult :type "HitResult Structure (by ref)"))
  (bind _asbp_player (cast `/Game/Characters/Player/BP_Player` OtherActor))
  (set `self.Player Ref` _asbp_player))

(event `self.Box.OnComponentEndOverlap`
  (params (OverlappedComponent :type "PrimitiveComponent Object Reference") (OtherActor :type "Actor Object Reference") (OtherComp :type "PrimitiveComponent Object Reference") (OtherBodyIndex :type Integer))
  (cast `/Game/Characters/Player/BP_Player` OtherActor)
  (set `self.Player Ref` null))

(fn `UserConstructionScript`)