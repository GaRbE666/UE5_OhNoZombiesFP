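; Buyable perk machine that grants the player Juggernaut, Speed Cola, Stamin Up or Quick Revive, selected by an enum.
; Box overlap caches the player, enables purchasing for unowned perks and shows a prompt widget.
; Tick polls for interaction, sufficient points and no reload or ADS, then sets that perk's flag on the player.
; All perks except Quick Revive require BP_Light to be on; Quick Revive has limited uses.
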(event `self.ReceiveBeginPlay`
  (bind _returnvalue (`GameplayStatics.GetActorOfClass` "/Game/Blueprints/IteractableItems/BP_Light.BP_Light_C"))
  (set `self.BP Light Ref` _returnvalue))

(event `self.ReceiveTick`
  (params (DeltaSeconds :type "Float (single-precision)"))
  (bind _player_ref (`self.Player Ref`))
  (`/Engine/EditorBlueprintResources/StandardMacros.IsValid` (`self.Player Ref`)
    (:`Is Valid`
      (if (or (`/Game/Blueprints/IteractableItems/BP_Light.LightIsOn` (`self.BP Light Ref`)) (`|EnumEquality` (`self.PerksEnum`) "NewEnumerator3"))
        ;[1 1 1] Checks
        (if (and (`/Game/Characters/Player/BP_Player.isInteracting` _player_ref) (`/Game/Characters/Player/BP_Player.canSpendPoints` _player_ref) (>= (`/Game/Characters/Player/BP_Player.Points` (`self.Player Ref`)) (`self.Perk Cost`)))
          (if (and (`KismetSystemLibrary.IsValid` (`self.Player Ref`)) (not (`/Game/Characters/Player/BP_Player.isReloading` (`self.Player Ref`))) (not (`/Game/Characters/Player/BP_Player.isADS` (`self.Player Ref`))))
            (switch `/Game/Blueprints/PerksEnum` (`self.PerksEnum`)
              (:`NewEnumerator0`
                ;[1 1 1] Juggernaut
                (set `/Game/Characters/Player/BP_Player.JugIsActivated` true (`self.Player Ref`))
                (`/Game/Blueprints/Components/BPC_Health.Update Max Health` (`/Game/Characters/Player/BP_Player.BPC_Health` (`self.Player Ref`)))
                (set `/Game/Characters/Player/BP_Player.canSpendPoints` false (`self.Player Ref`) :!label _label)
                (`Widget.RemoveFromParent` (`self.WB Text Ref`)))
              (:`NewEnumerator1`
                ;[1 1 1] Speed cola
                (set `/Game/Characters/Player/BP_Player.SpeedCActivated` true (`self.Player Ref`))
                (goto _label))
              (:`NewEnumerator2`
                ;[1 1 1] Stamin Up
                (set `/Game/Characters/Player/BP_Player.StaminUpActivated` true (`self.Player Ref`))
                (goto _label))
              (:`NewEnumerator3`
                ;[1 1 1] Quick Revive
                (if (> (`/Game/Characters/Player/BP_Player.QuickRevLeft` (`self.Player Ref`)) 0)
                  (set `/Game/Characters/Player/BP_Player.QuickRevActivated` true (`self.Player Ref`))
                  (`/Engine/EditorBlueprintResources/StandardMacros.DecrementInt` (`/Game/Characters/Player/BP_Player.QuickRevLeft` (`self.Player Ref`))
                    (:`  `
                      (goto _label))))))))))))

(event `self.Box.OnComponentBeginOverlap`
  (params (OverlappedComponent :type "PrimitiveComponent Object Reference") (OtherActor :type "Actor Object Reference") (OtherComp :type "PrimitiveComponent Object Reference") (OtherBodyIndex :type Integer) (bFromSweep :type Boolean) (SweepResult :type "HitResult Structure (by ref)"))
  (bind _asbp_player (cast `/Game/Characters/Player/BP_Player` OtherActor))
  (set `self.Player Ref` _asbp_player)
  (switch `/Game/Blueprints/PerksEnum` (`self.PerksEnum`)
    (:`NewEnumerator0`
      (if (not (`/Game/Characters/Player/BP_Player.JugIsActivated` (`self.Player Ref`)))
        (set `/Game/Characters/Player/BP_Player.canSpendPoints` true (`self.Player Ref`) :!label _label_2)
        (`self.Show Text`)))
    (:`NewEnumerator1`
      (if (not (`/Game/Characters/Player/BP_Player.SpeedCActivated` (`self.Player Ref`)))
        (goto _label_2)))
    (:`NewEnumerator2`
      (if (not (`/Game/Characters/Player/BP_Player.StaminUpActivated` (`self.Player Ref`)))
        (goto _label_2)))
    (:`NewEnumerator3`
      (if (not (`/Game/Characters/Player/BP_Player.QuickRevActivated` (`self.Player Ref`)))
        (goto _label_2)))))

(event `self.Box.OnComponentEndOverlap`
  (params (OverlappedComponent :type "PrimitiveComponent Object Reference") (OtherActor :type "Actor Object Reference") (OtherComp :type "PrimitiveComponent Object Reference") (OtherBodyIndex :type Integer))
  (bind _asbp_player (cast `/Game/Characters/Player/BP_Player` OtherActor))
  (set `self.Player Ref` null)
  (set `/Game/Characters/Player/BP_Player.canSpendPoints` false _asbp_player)
  (`/Engine/EditorBlueprintResources/StandardMacros.IsValid` (`self.WB Text Ref`)
    (:`Is Valid`
      (`Widget.RemoveFromParent` (`self.WB Text Ref`)))))

(fn `Show Text`
  (bind _returnvalue (`|CreateWidget` "/Game/Blueprints/Widgets/WB_Text.WB_Text_C"))
  (set `self.WB Text Ref` _returnvalue)
  (`UserWidget.AddToViewport` _returnvalue 0)
  (if (or (`/Game/Blueprints/IteractableItems/BP_Light.LightIsOn` (`self.BP Light Ref`)) (`|EnumEquality` (`self.PerksEnum`) "NewEnumerator3"))
    (if (and (== (`/Game/Characters/Player/BP_Player.QuickRevLeft` (`self.Player Ref`)) 0) (`|EnumEquality` (`self.PerksEnum`) "NewEnumerator3"))
      (`TextBlock.SetText` (`/Game/Blueprints/Widgets/WB_Text.BuyableText` (`self.WB Text Ref`)) "I think you've had too much of this!")
      (else
        (`TextBlock.SetText` (`/Game/Blueprints/Widgets/WB_Text.BuyableText` (`self.WB Text Ref`)) (`|FormatText` "Press F to buy {PerkName} ({PerkCost})" (`self.Perk Name`) (`self.Perk Cost`)))))
    (else
      (`TextBlock.SetText` (`/Game/Blueprints/Widgets/WB_Text.BuyableText` (`self.WB Text Ref`)) "You must first turn on the power"))))

(fn `UserConstructionScript`
  (`StaticMeshComponent.SetStaticMesh` (`self.StaticMesh`) (`self.Mesh`)))