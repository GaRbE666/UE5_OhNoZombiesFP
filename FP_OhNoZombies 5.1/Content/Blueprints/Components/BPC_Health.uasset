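; Health component that tracks an owner's current and maximum health, starting at full on BeginPlay.
; AddHealth and RemoveHealth clamp the value between zero and max, with RemoveHealth returning whether health has run out.
; On Tick, only player-owned instances regenerate, using a time accumulator to restore a small fixed amount at a steady interval while below max.
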(event `self.ReceiveBeginPlay`
  (set `self.Current Health` (`self.Max Health`)))

(event `self.ReceiveTick`
  (params (DeltaSeconds :type "Float (single-precision)"))
  (bind _returnvalue (+ DeltaSeconds (`self.Time To Recover Health`)))
  ;[1 1 1] Recover Health by time
  (cast `/Game/Characters/Player/BP_Player` (`self.GetOwner`))
  (if (< (`self.Current Health`) (`self.Max Health`))
    (set `self.canRecoverHealth` true)
    (else
      (set `self.canRecoverHealth` false)))
  (if (`self.canRecoverHealth`)
    (if (>= _returnvalue 0.25)
      (set `self.Time To Recover Health` 0.0)
      (`self.Add Health` 1.0)
      (else
        (set `self.Time To Recover Health` _returnvalue)))))

(fn `Add Health`
  (params (Amount :type "Float (double-precision)"))
  (set `self.Current Health` (`KismetMathLibrary.FClamp` (+ Amount (`self.Current Health`)) 0.0 (`self.Max Health`))))

(fn `Remove Health`
  (params (Amount :type "Float (double-precision)"))
  (returns (Dead :type Boolean))
  (bind _output_get (set `self.Current Health` (`KismetMathLibrary.FClamp` (- (`self.Current Health`) Amount) 0.0 (`self.Max Health`))))
  (return (<= _output_get 0.0)))