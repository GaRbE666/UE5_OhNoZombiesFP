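; GM_Zombies is a game mode that runs endless rounds of zombie waves with rising zombie count and health.
; Each round raises capped max health, linearly then by percentage, waits, then derives the wave size from round number and level limit.
; A looping timer spawns zombies through random BP_ZombieSpawner actors, throttled by live zombie count.
; Tick starts the next round once all have spawned and the externally updated death count matches the total.
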(event `self.ReceiveBeginPlay`
  (`self.IncreaseRound`))

(event `self.ReceiveTick`
  (params (DeltaSeconds :type "Float (single-precision)"))
  (if (`self.Spawned All Zombies`)
    (if (== (`self.Zombies Dead`) (`self.Total Zombies In Round`))
      (`self.IncreaseRound`))))

(event `IncreaseRound`
  (set `self.Spawned All Zombies` false)
  (`/Engine/EditorBlueprintResources/StandardMacros.IncrementInt` (`self.Round Number`)
    (:`  `
      (set `self.Zombies Dead` 0)
      ;[1 1 1] Select max health zombie depending of Round
      (set `self.Max Health` (`KismetMathLibrary.Clamp` (select `bool` (< (`self.Round Number`) 10) :`false` (`KismetMathLibrary.FTrunc` (* (`self.Max Health`) 1.1)) :`true` (+ (`self.Max Health`) 100)) 0 10000))
      (`KismetSystemLibrary.Delay` (`self.Time Between Rounds`))
      (`self.StartRound`))))

(event `StartRound`
  (set `self.Total Zombies In Round` (select `bool` (== (`self.Round Number`) 1) :`false` (`KismetMathLibrary.Round` (* (* (`self.Round Number`) 0.15) (`self.Max Zombies In Level`))) :`true` 6))
  (bind _returnvalue (`KismetSystemLibrary.K2_SetTimerDelegate` (delegate `SpawnZombie`) (`self.Time Between Each Spawn`) true)))

(event `SpawnZombie`
  (if (< (`self.Zombie Spawned`) (`self.Total Zombies In Round`))
    (bind _outactors (`GameplayStatics.GetAllActorsOfClass` "/Game/Characters/Zombie/Blueprints/BP_AI_Zombie.BP_AI_Zombie_C"))
    (if (<= (`KismetArrayLibrary.Array_Length` _outactors) (`self.Max Zombies In Level`))
      ;[1 1 1] Select Random Spawner
      (bind _outactors_2 (`GameplayStatics.GetAllActorsOfClass` "/Game/Blueprints/BP_ZombieSpawner.BP_ZombieSpawner_C"))
      (`/Game/Blueprints/BP_ZombieSpawner.Spawn` (`|GetArrayItem` _outactors_2 (`KismetMathLibrary.RandomIntegerInRange` 0 (- (`KismetArrayLibrary.Array_Length` _outactors_2) 1))) (`KismetMathLibrary.Conv_IntToDouble` (`self.Max Health`)))
      (`/Engine/EditorBlueprintResources/StandardMacros.IncrementInt` (`self.Zombie Spawned`)))
    (else
      (`KismetSystemLibrary.K2_ClearAndInvalidateTimerHandle` (stale `StartRound` _returnvalue))
      (set `self.Zombie Spawned` 0)
      (set `self.Spawned All Zombies` true))))

(fn `UserConstructionScript`)