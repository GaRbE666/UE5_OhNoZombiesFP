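; AI controller for zombie characters that runs the BT_Zombie behavior tree after a short delay on BeginPlay, holding off the walk.
; Every tick it checks whether the controlled pawn is within close range of the first player character and writes the result to the InAttackRange blackboard key.
; The range is a hardcoded distance threshold, polled in the controller itself.
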(event `self.ReceiveBeginPlay`
  ;[1 1 1] Delay before Zombie walk
  (`KismetSystemLibrary.Delay` 1.0)
  (`self.RunBehaviorTree` "/Game/Characters/Zombie/Blueprints/BT_Zombie.BT_Zombie"))

(event `self.ReceiveTick`
  (params (DeltaSeconds :type "Float (single-precision)"))
  (`/Engine/EditorBlueprintResources/StandardMacros.IsValid` (`AIBlueprintHelperLibrary.GetBlackboard` null)
    (:`Is Valid`
      (`BlackboardComponent.SetValueAsBool` (`AIBlueprintHelperLibrary.GetBlackboard` null) "InAttackRange" (< (`self.GetDistanceTo` (`self.K2_GetPawn`) (`GameplayStatics.GetPlayerCharacter` 0)) 125.0)))))

(fn `UserConstructionScript`)