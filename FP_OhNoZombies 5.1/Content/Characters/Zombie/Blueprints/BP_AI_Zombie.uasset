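; Zombie enemy character that hurts the player on contact and takes location-based damage.
; A sphere overlap damages BP_Player while CanDamage is set.
; TakeDamage scales hits by bone, reducing leg hits and boosting headshots, then passes them to BPCHealth.
; On death it ragdolls with an impulse from the negated impact point, increments GM_Zombies' dead count and expires after a short lifespan.
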(event `self.Sphere.OnComponentBeginOverlap`
  (params (OverlappedComponent :type "PrimitiveComponent Object Reference") (OtherActor :type "Actor Object Reference") (OtherComp :type "PrimitiveComponent Object Reference") (OtherBodyIndex :type Integer) (bFromSweep :type Boolean) (SweepResult :type "HitResult Structure (by ref)"))
  (if (`self.canDamage`)
    (bind _asbp_player (cast `/Game/Characters/Player/BP_Player` OtherActor))
    (`/Game/Characters/Player/BP_Player.Take Damage` _asbp_player 10.0 self)))

(fn `TakeDamage`
  (params (Amount :type "Float (double-precision)") (`Bone Name` :type Name) (`Impact Point` :type "Vector Structure"))
  (returns (dead :type Boolean))
  (bind _dead (`/Game/Blueprints/Components/BPC_Health.Remove Health` (`self.BPC_Health`) (select `bool` (or (== `Bone Name` "calf_l") (== `Bone Name` "calf_r") (== `Bone Name` "foot_l") (== `Bone Name` "foot_r") (== `Bone Name` "thigh_l") (== `Bone Name` "thigh_r")) :`false` (select `bool` (== `Bone Name` "head") :`false` Amount :`true` (* Amount 2.0)) :`true` (* Amount 0.8))))
  (if _dead
    ;[1 1 1] Physic Death
    (`PrimitiveComponent.SetSimulatePhysics` (`self.Mesh`) true)
    (`PrimitiveComponent.SetCollisionEnabled` (`self.CapsuleComponent`) "NoCollision")
    (`PrimitiveComponent.SetCollisionResponseToChannel` (`self.Mesh`) "ECC_Visibility" "ECR_Ignore")
    (`PrimitiveComponent.AddImpulse` (`self.Mesh`) (* `Impact Point` -10000.0) `Bone Name` false)
    (bind _asgm_zombies (cast `/Game/Blueprints/GameModes/GM_Zombies` (`GameplayStatics.GetGameMode`)))
    (`/Engine/EditorBlueprintResources/StandardMacros.IncrementInt` (`/Game/Blueprints/GameModes/GM_Zombies.Zombies Dead` _asgm_zombies)
      (:`  `
        (`self.SetLifeSpan` 10.0)
        (return true)))))

(fn `UserConstructionScript`)